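; Ground fire VFX actor that drives the direction of a Niagara fire effect from an angle.
; CalculateDirection prints DirAngle, then uses a chain of range checks to map it to hand-picked X and Y values per sector.
; SetDirection passes X and Y, with Z fixed at one, to the Direction variable on NSGroundFire.
; The event graph and construction script are empty, so neither function is called within this Blueprint.
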(event EventBeginPlay)

(event Collision|EventActorBeginOverlap
  (params (OtherActor :type Actor%20Object%20Reference)))

(event EventTick
  (params (DeltaSeconds :type Float%20%28single-precision%29)))

(fn ConstructionScript)

(fn CalculateDirection
  (Development|PrintString (Utilities|String|ToString(Float) (Variables|Default|GetDirAngle)))
  (if (and (>= (Variables|Default|GetDirAngle) 3e+01) (< (Variables|Default|GetDirAngle) 6e+01))
    (Variables|Default|Setx 1.0)
    (Variables|Default|Sety -1.0)
    (elif (and (>= (Variables|Default|GetDirAngle) 6e+01) (< (Variables|Default|GetDirAngle) 1.2e+02))
      (Variables|Default|Setx 1.5)
      (Variables|Default|Sety -1.0)
      (elif (and (>= (Variables|Default|GetDirAngle) 1.2e+02) (< (Variables|Default|GetDirAngle) 1.5e+02))
        (Variables|Default|Setx 1.0)
        (Variables|Default|Sety 0.0)
        (elif (and (>= (Variables|Default|GetDirAngle) 1.5e+02) (< (Variables|Default|GetDirAngle) 1.8e+02))
          (Variables|Default|Setx 1.0)
          (Variables|Default|Sety 1.0)
          (elif (and (>= (Variables|Default|GetDirAngle) 1.8e+02) (< (Variables|Default|GetDirAngle) 2.1e+02))
            (Variables|Default|Setx -1.0)
            (Variables|Default|Sety 1.0)
            (elif (and (>= (Variables|Default|GetDirAngle) 2.1e+02) (< (Variables|Default|GetDirAngle) 241.0))
              (Variables|Default|Setx -1.5)
              (Variables|Default|Sety 1.0)
              (elif (and (>= (Variables|Default|GetDirAngle) 241.0) (< (Variables|Default|GetDirAngle) 3e+02))
                (Variables|Default|Setx -2.0)
                (Variables|Default|Sety 1.0)
                (elif (and (>= (Variables|Default|GetDirAngle) 3e+02) (< (Variables|Default|GetDirAngle) 3.3e+02))
                  (Variables|Default|Setx -1.0)
                  (Variables|Default|Sety 0.0)
                  (elif (or (and (>= (Variables|Default|GetDirAngle) 3.3e+02) (< (Variables|Default|GetDirAngle) 3.6e+02)) (and (>= (Variables|Default|GetDirAngle) 0.0) (< (Variables|Default|GetDirAngle) 3e+01)))
                    (Variables|Default|Setx 0.0)
                    (Variables|Default|Sety -1.0)))))))))))

(fn SetDirection
  (Niagara|SetNiagaraVariable(Vector3) (Variables|Default|GetNS_groundFire) "Direction" (Math|Vector|MakeVector (Variables|Default|Getx) (Variables|Default|Gety) 1.0)))